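; Tank Blueprint that handles player turret-aiming input by rotating its camera boom.
; The Elevate_Turret and Rotate_Turret axes add local pitch and yaw to CameraBoom, scaled by world delta seconds and the WorldDeltaPad multiplier for frame-rate-independent speed.
; Only the boom is rotated in this graph, with no turret mesh movement or pitch clamping, and BeginPlay and the construction script are empty.
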(event `self.ReceiveBeginPlay`)

(event `InputAxis|Elevate_Turret`
  (params (AxisValue :type "Float (single-precision)"))
  ;[1 1 1] Turrent Elevation Input
  (`SceneComponent.K2_AddLocalRotation` (`self.CameraBoom`) (`KismetMathLibrary.MakeRotator` 0.0 (* AxisValue (`GameplayStatics.GetWorldDeltaSeconds`) (`self.WorldDeltaPad`))) false false))

(event `InputAxis|Rotate_Turret`
  (params (AxisValue :type "Float (single-precision)"))
  ;[1 1 1] Turret Rotate Input
  (`SceneComponent.K2_AddLocalRotation` (`self.CameraBoom`) (`KismetMathLibrary.MakeRotator` 0.0 0.0 (* AxisValue (`GameplayStatics.GetWorldDeltaSeconds`) (`self.WorldDeltaPad`))) false false))

(fn `UserConstructionScript`)